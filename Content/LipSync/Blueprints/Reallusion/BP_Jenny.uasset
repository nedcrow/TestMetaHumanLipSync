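; BP_Jenny is a talking character that lip-syncs speech and tracks the mouse cursor.
; OVRLipSync playback maps visemes to skeletal mesh morph targets, fed by preset voice clips with baked sequences or by text sent to MindsLab TTS and processed at runtime.
; Tick computes look-at targets: the head follows the cursor while left mouse is held, otherwise it eases back as the eyes track the cursor within clamped bounds.
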(event `self.OVRLipSyncPlaybackActor.OnVisemesReady`
  (bind _ovrlipsyncplaybackactor (`self.OVRLipSyncPlaybackActor`))
  ;[1 1 1] OVRLip
  (`OVRLipSyncActorComponentBase.AssignVisemesToMorphTargets` :`self` _ovrlipsyncplaybackactor :`Mesh` (`self.SkeletalMesh`))
  (set `self.visemes` (`KismetMathLibrary.Conv_IntToDouble` (`KismetArrayLibrary.Array_Length` (`OVRLipSyncActorComponentBase.GetVisemes` _ovrlipsyncplaybackactor)))))

(event `ClickedLipSync`
  (params (sampleIndex :type Integer))
  (bind _ovrlipsyncplaybackactor (`self.OVRLipSyncPlaybackActor`))
  (bind _audio (`self.Audio`))
  ;[1 1 1] OVRLip
  (switch `int` sampleIndex
    (:`0`
      (`AudioComponent.SetSound` _audio "/Game/Audio/voice_french_ttortia.voice_french_ttortia")
      (`OVRLipSyncPlaybackActorComponent.Start` _ovrlipsyncplaybackactor (`self.Audio`) "/Game/Audio/voice_french_ttortia_LipSyncSequence.voice_french_ttortia_LipSyncSequence"))
    (:`1`
      (`AudioComponent.SetSound` _audio "/Game/Audio/voice_hunmin.voice_hunmin")
      (`OVRLipSyncPlaybackActorComponent.Start` _ovrlipsyncplaybackactor (`self.Audio`) "/Game/Audio/voice_hunmin_LipSyncSequence.voice_hunmin_LipSyncSequence"))
    (:`2`
      (`AudioComponent.SetSound` _audio "/Game/Audio/voice_thankyou.voice_thankyou")
      (`OVRLipSyncPlaybackActorComponent.Start` _ovrlipsyncplaybackactor (`self.Audio`) "/Game/Audio/voice_thankyou_LipSyncSequence.voice_thankyou_LipSyncSequence"))
    (:`3`
      (`AudioComponent.SetSound` _audio "/Game/Audio/vox_lp_01.vox_lp_01")
      (`OVRLipSyncPlaybackActorComponent.Start` _ovrlipsyncplaybackactor (`self.Audio`) "/Game/Audio/vox_lp_01_LipSyncSequence.vox_lp_01_LipSyncSequence"))))

(event `self.ReceiveBeginPlay`
  ;[1 1 1] LipSync_TTS
  (add `TTSComponentWithMindsLab.TTSEvent` (`self.TTSComponentWithMindsLab`) (delegate `PostSuccessTTS`)))

(event `PostSuccessTTS`
  (params (SoundParameter :type "SoundWave Object Reference"))
  (bind _lipsynccomponentwithovr (`self.LipSyncComponentWithOVR`))
  (bind _audio (`self.Audio`))
  ;[1 1 1] LipSync_TTS
  (bind _returnvalue (`LipSyncComponentWithOVR.OVRLipSyncProcessSoundWave` _lipsynccomponentwithovr SoundParameter false))
  (if _returnvalue
    (set `AudioComponent.Sound` SoundParameter _audio)
    (`OVRLipSyncPlaybackActorComponent.Start` (`self.OVRLipSyncPlaybackActor`) _audio (`LipSyncComponentWithOVR.LipSyncSequence` _lipsynccomponentwithovr))))

(event `LipSyncFromText`
  (params (TargetText :type String))
  ;[1 1 1] LipSync_TTS
  (`KismetSystemLibrary.PrintString` TargetText)
  (`TTSComponentWithMindsLab.CallTTS` (`self.TTSComponentWithMindsLab`) TargetText))

(event `self.ReceiveTick`
  (params (DeltaSeconds :type "Float (single-precision)"))
  (bind (_cursorlocation_eyes_x _cursorlocation_eyes_y _cursorlocation_eyes_z) (`KismetMathLibrary.BreakVector` (`self.CursorLocation_Eyes`)))
  (bind (_cursorlocation_head_x _cursorlocation_head_y _cursorlocation_head_z) (`KismetMathLibrary.BreakVector` (`self.CursorLocation_Head`)))
  (bind (_cursorlocation_head_x_2 _cursorlocation_head_y_2) (`KismetMathLibrary.BreakVector` (`self.CursorLocation_Head`)))
  (bind _hitresult (`PlayerController.GetHitResultUnderCursorByChannel` (`GameplayStatics.GetPlayerController` 0) "TraceTypeQuery1" true))
  ;[1 1 1] Interaction_LookAtCursor
  (if (`self.IsClickedMouseL`)
    (set `self.CursorLocation_Head` (`.Location` (`GameplayStatics.BreakHitResult` _hitresult)))
    (else
      (set `self.CursorLocation_Head` (+ (`self.CursorLocation_Head`) (`KismetMathLibrary.MakeVector` 0.0 (* (/ _cursorlocation_head_y_2 (`self.RotSpeed`)) -1.0))))
      (set `self.CursorLocation_Head` (- (`self.CursorLocation_Head`) (`KismetMathLibrary.MakeVector` 0.0 0.0 (/ (- _cursorlocation_head_z 150.0) (`self.RotSpeed`)))))
      (set `self.CursorLocation_Eyes` (`.Location` (`GameplayStatics.BreakHitResult` _hitresult)))
      (set `self.CursorLocation_Eyes` (`KismetMathLibrary.MakeVector` 150.0 (`KismetMathLibrary.FClamp` _cursorlocation_eyes_y -50.0 50.0) (`KismetMathLibrary.FClamp` _cursorlocation_eyes_z 120.0 200.0)))
      (set `self.TempLocation` (`.Location` (`GameplayStatics.BreakHitResult` _hitresult))))))

(fn `UserConstructionScript`)