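; BP_LipSyncCameraPawn is a pawn for the lip sync feature that relays left mouse button input to character actors.
; On press and release it finds the first BP_Vivian, BP_Jenny and BP_LipSyncModelReallusion with GetActorOfClass, skipping any that are missing.
; It sets IsClickedMouseL on Vivian and Jenny, and Triggerd on the Reallusion model, true while held and false on release.
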(event `self.ReceiveBeginPlay`)

(event `Key|LeftMouseButton`
  (params (Key :type "Key Structure"))
  (:`Pressed`
    ;[1 1 1] ViVian
    (bind _returnvalue (`GameplayStatics.GetActorOfClass` "/Game/LipSync/Blueprints/Metahuman/BP_Vivian.BP_Vivian_C"))
    (if (`KismetSystemLibrary.IsValid` _returnvalue)
      (set `/Game/LipSync/Blueprints/Metahuman/BP_Vivian.IsClickedMouseL` true _returnvalue))
    ;[1 1 1] Jenny
    (bind _returnvalue_2 (`GameplayStatics.GetActorOfClass` "/Game/LipSync/Blueprints/Reallusion/BP_Jenny.BP_Jenny_C"))
    (if (`KismetSystemLibrary.IsValid` _returnvalue_2)
      (set `/Game/LipSync/Blueprints/Reallusion/BP_Jenny.IsClickedMouseL` true _returnvalue_2))
    ;[1 1 1] Reallusion
    (bind _returnvalue_3 (`GameplayStatics.GetActorOfClass` "/Game/LipSync/Blueprints/Refactorung/BP_LipSyncModelReallusion.BP_LipSyncModelReallusion_C"))
    (if (`KismetSystemLibrary.IsValid` _returnvalue_3)
      (set `LipSyncModelReallusion.bTriggerd` true _returnvalue_3)))
  (:`Released`
    (bind _returnvalue_4 (`GameplayStatics.GetActorOfClass` "/Game/LipSync/Blueprints/Metahuman/BP_Vivian.BP_Vivian_C"))
    (if (`KismetSystemLibrary.IsValid` _returnvalue_4)
      (set `/Game/LipSync/Blueprints/Metahuman/BP_Vivian.IsClickedMouseL` false _returnvalue_4))
    (bind _returnvalue_5 (`GameplayStatics.GetActorOfClass` "/Game/LipSync/Blueprints/Reallusion/BP_Jenny.BP_Jenny_C"))
    (if (`KismetSystemLibrary.IsValid` _returnvalue_5)
      (set `/Game/LipSync/Blueprints/Reallusion/BP_Jenny.IsClickedMouseL` false _returnvalue_5))
    (bind _returnvalue_6 (`GameplayStatics.GetActorOfClass` "/Game/LipSync/Blueprints/Refactorung/BP_LipSyncModelReallusion.BP_LipSyncModelReallusion_C"))
    (if (`KismetSystemLibrary.IsValid` _returnvalue_6)
      (set `LipSyncModelReallusion.bTriggerd` false _returnvalue_6))))

(fn `UserConstructionScript`)